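; Base animal that wanders, stares, flees, attacks, fetches sticks or seeks food, and can be petted, fed or captured.
; A sense sphere tracks a seen player and pickup, re-evaluating reactions on overlap changes and every Tick.
; Reactions choose a state from demeanor, Friendliness and distance, writing it to the AI controller's Blackboard.
; Friendliness thresholds per demeanor gate interactions, while petting and feeding raise Friendliness.
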(event OnComponentBeginOverlap(Sense)
  (params (OverlappedComponent :type Primitive%20Component%20Object%20Reference) (OtherActor :type Actor%20Object%20Reference) (OtherComp :type Primitive%20Component%20Object%20Reference) (OtherBodyIndex :type Integer) (bFromSweep :type Boolean) (SweepResult :type Hit%20Result%20Structure%20%28by%20ref%29))
  (bind _asplayer_character (Utilities|Casting|CastToPlayerCharacter OtherActor)
    (:then
      (bind _output_get (Variables|Senses|SetSeenPlayer _asplayer_character))
      (Development|PrintString "I see  you.")
      (AI|ReacttoPlayer _output_get true))
    (:CastFailed
      (bind _aspickup (Utilities|Casting|CastToPickup OtherActor))
      (bind _output_get_2 (Variables|Senses|SetSeenObject _aspickup))
      (AI|ReacttoPickup _output_get_2 true)
      (Development|PrintString "Whats that?"))))

(event OnComponentEndOverlap(Sense)
  (params (OverlappedComponent :type Primitive%20Component%20Object%20Reference) (OtherActor :type Actor%20Object%20Reference) (OtherComp :type Primitive%20Component%20Object%20Reference) (OtherBodyIndex :type Integer))
  (bind _asplayer_character (Utilities|Casting|CastToPlayerCharacter OtherActor)
    (:then
      (if (== _asplayer_character (Variables|Senses|GetSeenPlayer))
        (Variables|Senses|SetSeenPlayer 0)
        (Development|PrintString "Where did you go?")
        (AI|ReacttoPlayer 0 false)))
    (:CastFailed
      (bind _aspickup (Utilities|Casting|CastToPickup OtherActor))
      (if (== _aspickup (Variables|Senses|GetSeenObject))
        (Variables|Senses|SetSeenObject 0)
        (AI|ReacttoPickup 0 false)
        (Development|PrintString "Where did it go?")))))

(event EventTick
  (params (DeltaSeconds :type Float%20%28single-precision%29))
  (bind _seenplayer (Variables|Senses|GetSeenPlayer))
  (bind _seenobject (Variables|Senses|GetSeenObject))
  (Utilities|IsValid _seenplayer
    (:Is%20Valid
      (AI|ReacttoPlayer _seenplayer true))
    (:Is%20Not%20Valid
      _))
  (Utilities|IsValid _seenobject
    (:Is%20Valid
      (AI|ReacttoPickup _seenobject true))))

(fn ConstructionScript
  (bind _animalsenseradius (Variables|Traits|GetAnimalSenseRadius))
  (Components|Sphere|SetSphereRadius (Variables|Default|GetSense) (Variables|Traits|GetAnimalSenseRadius) true)
  (Variables|Traits|Reactions|SetStareRange (Utilities|Select :Index (Variables|Traits|GetAnimalDemeanor) :NewEnumerator0 0.0 :NewEnumerator1 _animalsenseradius :NewEnumerator2 _animalsenseradius)))

(fn TryCapture
  (params (Player :type Player%20Character%20Object%20Reference))
  (if (Utilities|CanCapture)
    (Animal|Capture|CaptureAnimal Player)
    (else
      (Development|PrintString "I dont like you!"))))

(fn CaptureAnimal
  (params (CapturingPlayer :type Player%20Character%20Object%20Reference))
  (Development|PrintString "You cought me!")
  (Actor|DestroyActor))

(fn GetFriendliness
  (return (Variables|Traits|GetFriendliness)))

(fn ModifyFriendliness
  (params (ValueChange :type Float%20%28single-precision%29))
  (Variables|Traits|SetFriendliness (+ ValueChange (Variables|Traits|GetFriendliness))))

(fn TryPet
  (if (Utilities|CanPet)
    (Development|PrintString "You pet the animal")
    (Animal|Friendliness|ModifyFriendliness 5.0)
    (else
      (Development|PrintString "I dont like you"))))

(fn TryFeed
  (if (Utilities|CanFeed)
    (Development|PrintString "NOM NOM NOM")
    (Animal|Feed|EatFood)
    (return true)
    (else
      (Development|PrintString "I don't like you.")
      (return false))))

(fn TryFetch
  (params (Player :type Player%20Character%20Object%20Reference) (Stick :type Pickup%20Object%20Reference))
  (if (Utilities|CanFetch)
    (Development|PrintString "I'll Get the stick!")
    (if (Utilities|Select :Index (AI|GetAnimalState) :NewEnumerator0 true :NewEnumerator1 true :NewEnumerator2 false :NewEnumerator3 false :NewEnumerator4 true :NewEnumerator5 true :NewEnumerator6 true)
      (Variables|Senses|SetSeenObject Stick)
      (AI|SetAnimalState "NewEnumerator4"))
    (else
      (Development|PrintString "I dont like you"))))

(fn SetController
  (params (AnimalController :type Animal%20AI%20Controller%20Object%20Reference))
  (Variables|References|SetAnimalControllerRef AnimalController))

(fn ReacttoPlayer
  (params (Player :type Player%20Character%20Object%20Reference) (CanSee :type Boolean))
  (LocalVariables|SetThePlayer Player)
  (LocalVariables|SetCanSeeThePlayer CanSee)
  (switch Utilities|FlowControl|Switch|SwitchonAnimalStates (AI|GetAnimalState)
    (:NewEnumerator0
      (if (LocalVariables|GetCanSeeThePlayer) :!label _label
        (Utilities|DoesAttack
          (:false
            (Utilities|DoesFlee
              (:false
                (Utilities|DoesStare (LocalVariables|GetThePlayer))))))))
    (:NewEnumerator1
      (if (LocalVariables|GetCanSeeThePlayer)
        (Utilities|DoesAttack
          (:true
            _)
          (:false
            (Utilities|DoesFlee
              (:true
                _))))
        (else
          (Utilities|DoesWander)))
      (AI|ClearFocus (Variables|References|GetAnimalControllerRef)))
    (:NewEnumerator2
      (if (not (LocalVariables|GetCanSeeThePlayer)) :!label _label_2
        (Utilities|DoesWander)))
    (:NewEnumerator3
      (goto _label_2))
    (:NewEnumerator4
      (goto _label))
    (:NewEnumerator5
      (goto _label))
    (:NewEnumerator6
      (if (not (LocalVariables|GetCanSeeThePlayer))
        (Utilities|DropItem)
        (Utilities|DoesWander)))))

(fn ReacttoPickup
  (params (Pickup :type Pickup%20Object%20Reference) (CanSee :type Boolean))
  (LocalVariables|SetPickupSeen Pickup)
  (LocalVariables|SetCanSeeIt CanSee)
  (switch Utilities|FlowControl|Switch|SwitchonAnimalStates (Variables|AI|GetAnimalState)
    (:NewEnumerator0
      (if (LocalVariables|GetCanSeeIt) :!label _label
        (Utilities|SetPickupBB (LocalVariables|GetPickupSeen))
        (Utilities|WhatIsPickup (LocalVariables|GetPickupSeen)
          (:Food
            (Utilities|DoesWantFood))
          (:Stick
            (Utilities|WillFetchforPlayer)))))
    (:NewEnumerator1
      (goto _label))
    (:NewEnumerator4
      (if (not (LocalVariables|GetCanSeeIt))
        (Utilities|SetPickupBB)
        (Utilities|DoesWander)))))

(fn EatFood
  (Animal|Friendliness|ModifyFriendliness 1e+01))

(fn SetAnimalState
  (params (NewAnimalState :type AnimalStates%20Enum))
  (bind _output_get (Variables|AI|SetAnimalState NewAnimalState))
  (AI|Components|Blackboard|SetValueasEnum (AI|GetBlackboard (Variables|References|GetAnimalControllerRef)) (Variables|References|Keys|GetAnimalStateKey) _output_get))

(fn GetAnimalState
  (return (Variables|AI|GetAnimalState)))

(fn DropPickup
  (Utilities|DropItem))

(fn PickupItem
  (params (Item :type Pickup%20Object%20Reference))
  (Utilities|Casting|CastToStickPickup Item
    (:then
      (bind _output_get (Variables|Default|SetHoldingItem Item))
      (Transformation|AttachActorToActor _output_get self "HoldSpot" "SnapToTarget" "SnapToTarget" "SnapToTarget" true))
    (:CastFailed
      (Actor|DestroyActor Item))))

(fn GetDemeanor
  (return (Variables|Traits|GetAnimalDemeanor)))

(fn WillFeed
  (return (Utilities|CanFeed)))

(fn WillFetch
  (return (Utilities|CanFetch)))

(fn WillPet
  (return (Utilities|CanPet)))