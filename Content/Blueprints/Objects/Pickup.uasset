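; Base pickup actor that the player collects into their inventory by walking into its radius.
; On BeginPlay it traces downward to settle on the ground, then disables static mesh collision.
; On overlap with a PlayerCharacter, a successful inventory add unregisters it from its spawner, hides it and flags it as picked up.
; UseItem is a placeholder that only prints the item's name.
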(event OnComponentBeginOverlap(PickupRadius)
  (params (OverlappedComponent :type Primitive%20Component%20Object%20Reference) (OtherActor :type Actor%20Object%20Reference) (OtherComp :type Primitive%20Component%20Object%20Reference) (OtherBodyIndex :type Integer) (bFromSweep :type Boolean) (SweepResult :type Hit%20Result%20Structure%20%28by%20ref%29))
  (bind _spawner (Variables|Default|GetSpawner))
  (bind _asplayer_character (Utilities|Casting|CastToPlayerCharacter OtherActor))
  (bind _success (Default|AddItemtoInventory _asplayer_character self))
  (if _success
    (Utilities|IsValid _spawner
      (:Is%20Valid
        (Default|RemoveItem _spawner self))
      (:Is%20Not%20Valid
        _))
    (Rendering|SetActorHiddenInGame true)
    (Collision|SetCollisionEnabled (Variables|Default|GetPickupRadius) "NoCollision")
    (Variables|Default|SetbIsPickedUp true)))

(event EventBeginPlay
  (bind _returnvalue (Transformation|GetActorLocation))
  (bind _returnvalue_2 (Transformation|GetActorLocation))
  (bind (_x _y _z) (Math|Vector|BreakVector _returnvalue))
  (bind (_x_2 _y_2 _z_2) (Math|Vector|BreakVector _returnvalue_2))
  ;[1 1 1] Set on ground
  (bind (_outhit _returnvalue_3) (Collision|LineTraceByChannel _returnvalue_2 (Math|Vector|MakeVector _x_2 _y_2 (- _z_2 1e+03)) "TraceTypeQuery1" false (Utilities|Array|MakeArray self) "None"))
  (if _returnvalue_3
    (Transformation|SetActorLocation (.Location (Collision|BreakHitResult _outhit)) true false)
    (Collision|SetCollisionEnabled (Variables|Default|GetStaticMesh) "NoCollision")
    (else
      (Transformation|SetActorLocation (Math|Vector|MakeVector _x _y (- _z 1e+03)) true false)
      (Collision|SetCollisionEnabled (Variables|Default|GetStaticMesh) "NoCollision"))))

(fn ConstructionScript)

(fn UseItem
  (Development|PrintString (Utilities|String|Append "Use: " (Utilities|GetDisplayName self))))