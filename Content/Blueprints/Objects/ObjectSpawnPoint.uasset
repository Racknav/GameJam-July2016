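; Spawn point actor that keeps an area stocked with pickups, up to a set count.
; A looping timer starts on BeginPlay and calls SpawnItem, placing pickups at random points inside a box sized in the construction script.
; The timer clears when SpawnItem finds the area full.
; Each pickup receives the spawner as a reference, and RemoveItem drops a pickup from the tracked list and restarts the timer.
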(event EventBeginPlay
  (Utilities|CreateTimer))

(fn ConstructionScript
  (Components|Box|SetBoxExtent (Variables|Default|GetBox) (Variables|SpawnOptions|GetBoxSize) true))

(fn RemoveItem
  (params (Pickup :type Pickup%20Object%20Reference))
  (Utilities|Array|RemoveItem (Variables|Default|GetItemsSpawned) Pickup)
  (Utilities|CreateTimer))

(fn SpawnItem
  (bind _box (Variables|Default|GetBox))
  (if (< (Utilities|Array|Length (Variables|Default|GetItemsSpawned)) (Variables|SpawnOptions|GetNumberToSpawn))
    (bind _returnvalue (Game|SpawnActorfromClass (Variables|SpawnOptions|GetPickupToSpawn) (Math|Transform|MakeTransform (Math|Random|RandomPointinBoundingBox (Transformation|GetWorldLocation _box) (Variables|/Script/Engine.BoxComponent|GetBoxExtent _box)) "0, 0, 0" "1,1,1") "AdjustIfPossibleButDontSpawnIfColliding" 0 self 0))
    (Utilities|Array|Add (Variables|Default|GetItemsSpawned) _returnvalue)
    (else
      (Utilities|Time|ClearandInvalidateTimerbyHandle (Variables|Default|GetSpawnTimerHandle)))))