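; StickPickup is a pickup item that a character can throw for animals to fetch.
; UseItem detaches and unhides the stick, enables physics and launches it along the character's pitched forward vector with random spin.
; It then flags the stick as thrown and for animals.
; Pickups before a throw use the parent logic, while later ones only call TryFetch on an AnimalBase.
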(event EventBeginPlay
  (|CallParentFunction))

(event EventPickupItem
  (params (Object :type Object%20Object%20Reference))
  (if (Variables|Default|GetThrown)
    (CallFunction|AnimalPickup Object)
    (else
      (|CallParentFunction Object))))

(fn ConstructionScript
  (|CallParentFunction))

(fn AnimalPickup
  (params (Object :type Object%20Object%20Reference))
  (bind _asanimal_base (Utilities|Casting|CastToAnimalBase Object))
  (Default|TryFetch _asanimal_base))

(fn UseItem
  (params (Character :type Player%20Character%20Object%20Reference))
  (Transformation|DetachFromActor "KeepWorld" "KeepWorld" "KeepWorld")
  (Rendering|SetActorHiddenInGame false)
  (Collision|SetCollisionEnabled (Variables|Default|GetStaticMesh) "QueryAndPhysics")
  (Physics|SetSimulatePhysics (Variables|Default|GetStaticMesh) true)
  (Physics|AddImpulse (Variables|Default|GetStaticMesh) (* (Math|Vector|RotateVector (Transformation|GetActorForwardVector Character) (Math|Rotator|MakeRotator 0.0 -45.0 0.0)) 8e+02) "None" true)
  (Class|PrimitiveComponent|SetPhysicsAngularVelocity (Variables|Default|GetStaticMesh) (* (Math|Random|RandomUnitVector) (Math|Random|RandomFloatinRange 5e+01 2e+02)) true "None")
  (Variables|Default|SetThrown true)
  (Variables|Default|SetbIsForAnimals true)
  (return true))